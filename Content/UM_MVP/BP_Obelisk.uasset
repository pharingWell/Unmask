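; BP_Obelisk is a poseable-mesh obelisk actor that the player rotates one bone at a time through input.
; The Bone input toggles between two bones and shifts a static mesh between two heights, while RotateL and RotateR turn the selected bone in small component-space steps.
; BeginPlay builds and stores a hard-coded keyframe sequence for Bone_001.
; The sequence comparison logic is disconnected, suggesting an unfinished pose-matching prototype.
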(event `EnhancedInput|/Game/TopDown/Input/Actions/IA_SetDestination_Click`
  (params (ActionValue :type Boolean) (ElapsedSeconds :type "Float (double-precision)") (TriggeredSeconds :type "Float (double-precision)") (InputAction :type "InputAction Object Reference" :default "/Game/TopDown/Input/Actions/IA_SetDestination_Click.IA_SetDestination_Click"))
  (:`Triggered`
    (`|PlayMontage` null
      (:`OnCompleted`
        (`KismetSystemLibrary.PrintString` "Finished")))))

(event `self.ReceiveBeginPlay`
  (`parent.ReceiveBeginPlay`)
  (bind _returnvalue (`UMAnimationProducer.CreateSequence` (`|MakeMap` "Bone_001" (make `UMJointTimeline` (`|MakeArray` (make `UMJointKey` 0.0 (`KismetMathLibrary.MakeTransform` (0.0 0.0 0.0))) (make `UMJointKey` 1.0 (`KismetMathLibrary.MakeTransform` (0.0 0.0 0.0) (struct :`Yaw` 90.0))) (make `UMJointKey` 2.0 (`KismetMathLibrary.MakeTransform` (0.0 0.0 0.0) (struct :`Pitch` 90.0 :`Roll` 90.0))) (make `UMJointKey` 3.0 (`KismetMathLibrary.MakeTransform` (0.0 0.0 0.0) (struct :`Roll` -90.0))) :!type "UMJointKey Structure")) :!type "Name" :!valuetype "UMJointTimeline Structure") (`SkinnedMeshComponent.SkeletalMesh` (`self.PoseableMesh`))))
  (set `self.Sequence` _returnvalue))

(event `InputAction|Bone`
  (params (Key :type "Key Structure"))
  (:`Released`
    (bind _isa (`/Engine/EditorBlueprintResources/StandardMacros.FlipFlop`)
      (:`A`
        _)
      (:`B`
        _))
    (set `self.Bone` (`KismetMathLibrary.SelectName` "Bone" "Bone_001" _isa))
    (`SceneComponent.K2_SetRelativeLocation` (`self.StaticMesh`) (`KismetMathLibrary.SelectVector` (-315.0 0.0 55.0) (-315.0 0.0 70.0) _isa) false true)))

(event `InputAction|RotateL`
  (params (Key :type "Key Structure"))
  (bind _bone (`self.Bone`))
  (bind (_returnvalue_location _returnvalue_rotation _returnvalue_scale) (`KismetMathLibrary.BreakTransform` (`SkinnedMeshComponent.GetBoneTransform` (`self.PoseableMesh`) _bone "RTS_Component")))
  (:`Pressed`
    (`PoseableMeshComponent.SetBoneTransformByName` (`self.PoseableMesh`) _bone (`KismetMathLibrary.MakeTransform` _returnvalue_location (`KismetMathLibrary.ComposeRotators` _returnvalue_rotation (struct :`Roll` -2.0)) _returnvalue_scale) "ComponentSpace")))

(event `InputAction|RotateR`
  (params (Key :type "Key Structure"))
  (bind _bone (`self.Bone`))
  (bind (_returnvalue_location _returnvalue_rotation _returnvalue_scale) (`KismetMathLibrary.BreakTransform` (`SkinnedMeshComponent.GetBoneTransform` (`self.PoseableMesh`) _bone "RTS_Component")))
  (:`Pressed`
    (`PoseableMeshComponent.SetBoneTransformByName` (`self.PoseableMesh`) _bone (`KismetMathLibrary.MakeTransform` _returnvalue_location (`KismetMathLibrary.ComposeRotators` _returnvalue_rotation (struct :`Roll` 2.0)) _returnvalue_scale) "ComponentSpace")))

(fn `UserConstructionScript`)
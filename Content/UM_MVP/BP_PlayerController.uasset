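; Player controller that spawns and possesses an animation editor character and manages Enhanced Input mapping contexts.
; On BeginPlay it applies the default context, spawns BP_AnimEditorCharacter at its own transform, possesses it and passes itself to InitializePawn.
; An EnterAnimEditor event switches immediately to the anim editor context.
; Helper functions wrap the input subsystem with validity checks; setting a context clears all existing mappings first.
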(event `self.ReceiveBeginPlay`
  (`self.Set Mapping Context` "/Game/UM_MVP/FirstPerson/Input/IMC_Default.IMC_Default")
  (bind _returnvalue (`|SpawnActorFromClass` "/Game/UM_MVP/AnimationEditor/BP_AnimEditorCharacter.BP_AnimEditorCharacter_C" (`self.GetTransform`) "AlwaysSpawn" "MultiplyWithRoot" null null))
  (`self.Possess` _returnvalue)
  (`/Game/UM_MVP/AnimationEditor/BP_AnimEditorCharacter.Initialize Pawn` _returnvalue self))

(event `Enter AnimEditor`
  (`self.Set Mapping Context` "/Game/UM_MVP/FirstPerson/Input/IMC_AnimEditor.IMC_AnimEditor" 0 (make `ModifyContextOptions` true true)))

(fn `Add Mapping Context`
  (params (MappingContext :type "InputMappingContext Object Reference") (Priority :type Integer) (Options :type "ModifyContextOptions Structure (by ref)"))
  (bind _returnvalue (subsystem `EnhancedInputLocalPlayerSubsystem`))
  (`/Engine/EditorBlueprintResources/StandardMacros.IsValid` _returnvalue
    (:`Is Valid`
      (`EnhancedInputSubsystemInterface.AddMappingContext` _returnvalue MappingContext Priority Options))))

(fn `Remove Mapping Context`
  (params (MappingContext :type "InputMappingContext Object Reference") (Options :type "ModifyContextOptions Structure (by ref)"))
  (bind _returnvalue (subsystem `EnhancedInputLocalPlayerSubsystem`))
  (`/Engine/EditorBlueprintResources/StandardMacros.IsValid` _returnvalue
    (:`Is Valid`
      (`EnhancedInputSubsystemInterface.RemoveMappingContext` _returnvalue MappingContext Options))))

(fn `Set Mapping Context`
  (params (MappingContext :type "InputMappingContext Object Reference") (Priority :type Integer) (Options :type "ModifyContextOptions Structure (by ref)"))
  (bind _returnvalue (subsystem `EnhancedInputLocalPlayerSubsystem`))
  (`/Engine/EditorBlueprintResources/StandardMacros.IsValid` _returnvalue
    (:`Is Valid`
      (`EnhancedInputSubsystemInterface.ClearAllMappings` _returnvalue)
      (`self.Add Mapping Context` MappingContext Priority Options))))

(fn `UserConstructionScript`)